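; Character fragment that adds a cosmetic actor to a Pekorobo character while the fragment is active.
; On begin, it spawns the configured CosmeticActor class and snaps it to the character's skeletal mesh component whose name matches AttachTo.
; The cosmetic's ABP_Pekorobo_CopyPose anim instance receives that mesh as its pose source.
; On end, it destroys the spawned actor.
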(event `self.OnBeginPlayFragment`
  (bind _cosmeticactor (`self.CosmeticActor`))
  (bind _returnvalue (`KismetSystemLibrary.Conv_InterfaceToObject` (`self.GetOwningCharacter`)))
  (`/Engine/EditorBlueprintResources/StandardMacros.IsValid` _returnvalue
    (:`Is Valid`
      (bind _asbp_character_pekorobo (cast `/Game/Characters/Pekorobo/BP_Character_Pekorobo` _returnvalue))
      (`|ExecutionSequence`
        (:`then_0`
          (if (`KismetSystemLibrary.IsValidClass` _cosmeticactor)
            (bind _returnvalue_2 (`BasicStuffBPFL.SpawnActor` _asbp_character_pekorobo _cosmeticactor (`KismetMathLibrary.MakeTransform` (0.0 0.0 0.0))))
            (bind _output_get (set `self.SpawnedActor` _returnvalue_2))
            (bind _foundskeletalmeshcomponent (`self.Find Skeletal Mesh for Name` _asbp_character_pekorobo (`self.AttachTo`)))
            (`Actor.K2_AttachToComponent` _output_get _foundskeletalmeshcomponent "None" "SnapToTarget" "SnapToTarget" "SnapToTarget" true)
            (bind _asb_character_cosmetic_pekorobo (cast `/Game/Characters/Pekorobo/B_CharacterCosmetic_Pekorobo` _output_get))
            (bind _asabp_pekorobo_copy_pose (cast `/Game/Characters/Pekorobo/ABP_Pekorobo_CopyPose` (`SkeletalMeshComponent.GetAnimInstance` (`/Game/Characters/Pekorobo/B_CharacterCosmetic_Pekorobo.SkeletalMesh` _asb_character_cosmetic_pekorobo))))
            (set `/Game/Characters/Pekorobo/ABP_Pekorobo_CopyPose.Source Mesh Component` _foundskeletalmeshcomponent _asabp_pekorobo_copy_pose)
            (else
              (`KismetSystemLibrary.PrintString` null "BP_CF_Pekorobo_Cosmetic: got invalid class"))))))))

(event `self.OnEndPlayFragment`
  (bind _spawnedactor (`self.SpawnedActor`))
  (bind _returnvalue (`KismetSystemLibrary.Conv_InterfaceToObject` (`self.GetOwningCharacter`)))
  (`/Engine/EditorBlueprintResources/StandardMacros.IsValid` _returnvalue
    (:`Is Valid`
      (cast `/Game/Characters/Pekorobo/BP_Character_Pekorobo` _returnvalue)
      (`/Engine/EditorBlueprintResources/StandardMacros.IsValid` _spawnedactor
        (:`Is Valid`
          (`Actor.K2_DestroyActor` _spawnedactor))))))

(fn `Find Skeletal Mesh for Name`
  (params (TargetActor :type "Actor Object Reference") (TargetSkelMeshCompName :type Name))
  (returns (FoundSkeletalMeshComponent :type "SkeletalMeshComponent Object Reference"))
  (for _array_element (`Actor.K2_GetComponentsByClass` TargetActor "/Script/Engine.SkeletalMeshComponent")
    (if (`KismetStringLibrary.EqualEqual_StrStr` (`KismetSystemLibrary.GetObjectName` _array_element) (`KismetStringLibrary.Conv_NameToString` TargetSkelMeshCompName))
      (return _array_element)))
  (return null))