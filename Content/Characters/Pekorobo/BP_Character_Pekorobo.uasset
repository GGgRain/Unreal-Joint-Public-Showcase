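; Pekorobo character Blueprint, usable by player or AI, with movement, run/grab ability input and dialogue skipping through Joint gameplay events.
; BeginPlay starts fragment objects, per-bone physical animation, input mapping and the unequipped anim layer.
; Speech synthesizer syllables drive vowel mouth morphs, while a looping timer turns AI bodies toward their eye gaze.
; Death explodes the mesh into an impulse-driven ragdoll with dust and sound, and Unexplode restores it.
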(event `self.BeginPlayFragments`
  (bind _outfragments (`self.GetFragments`))
  (for _array_element _outfragments
    (`CharacterFragment.BeginPlayFragment` _array_element)))

(event `self.ReceiveBeginPlay`
  (`|ExecutionSequence`
    (:`then_0`
      (`self.BeginPlayFragments`)
      (`self.Set Physical Animations` false))
    (:`then_1`
      (bind _asplayer_controller (cast `PlayerController` (`self.GetController`)))
      (`self.EnableInput` _asplayer_controller)
      (`/Game/Input/BPFL_InputHelper.BindMappingContextsForCharacter` (`self.Mapping Context`) self))
    (:`then_2`
      (`self.LinkAnimLayer` "/Game/Characters/Pekorobo/ABP_Pekorobo_ItemLayer_Unequipped.ABP_Pekorobo_ItemLayer_Unequipped_C")
      (`self.StartTickTimer` (delegate `TickTimerCB`)))))

(event `self.EndPlayFragments`
  (bind _outfragments (`self.GetFragments`))
  (for _array_element _outfragments
    (`CharacterFragment.EndPlayFragment` _array_element)))

(event `TickTimerCB`
  (if (`self.bAllowAIEyeTurning`)
    (if (not (or (`self.GetIsDead`) (not (`ActorComponent.IsActive` (`self.CharacterMovement`)))))
      (cast `AIController` (`self.GetController`))
      (for _array_element (`JointFacialAnimationComponent.EyeAnimationDataArray` (`self.JointFacialAnimation`))
        (`self.TurnInPlaceRate` (* (.yaw (`.TargetEyeGazeRotation` (break `JointEyeAnimationData` _array_element))) 0.5))))))

(event `self.BP_Joint_SpeechSynthesizer.OnSoundPlayed`
  (params (PlayedSyllable :type Name))
  ;[1 1 1] Speech Animation
  (switch `string` (`KismetStringLibrary.ToLower` (`KismetStringLibrary.Conv_NameToString` PlayedSyllable))
    (:`a`
      (`JointFacialAnimationComponent.StartFacialAnimation` (`self.JointFacialAnimation`) (make `JointFacialAnimationDefinition` "Mouth" true "Morph_Mouth_Speech_A" "/Game/Speech/CV_SpeechAnim.CV_SpeechAnim" 2.5 3.0 (`self.FacialAnimationDuration`) 0.99)))
    (:`e`
      (`JointFacialAnimationComponent.StartFacialAnimation` (`self.JointFacialAnimation`) (make `JointFacialAnimationDefinition` "Mouth" true "Morph_Mouth_Speech_E" "/Game/Speech/CV_SpeechAnim.CV_SpeechAnim" 2.5 2.0 (`self.FacialAnimationDuration`) 0.99)))
    (:`i`
      (`JointFacialAnimationComponent.StartFacialAnimation` (`self.JointFacialAnimation`) (make `JointFacialAnimationDefinition` "Mouth" true "Morph_Mouth_Speech_I" "/Game/Speech/CV_SpeechAnim.CV_SpeechAnim" 2.5 1.0 (`self.FacialAnimationDuration`) 0.99)))
    (:`o`
      (`JointFacialAnimationComponent.StartFacialAnimation` (`self.JointFacialAnimation`) (make `JointFacialAnimationDefinition` "Mouth" true "Morph_Mouth_Speech_O" "/Game/Speech/CV_SpeechAnim.CV_SpeechAnim" 2.0 1.0 (`self.FacialAnimationDuration`) 0.99)))
    (:`u`
      (`JointFacialAnimationComponent.StartFacialAnimation` (`self.JointFacialAnimation`) (make `JointFacialAnimationDefinition` "Mouth" true "Morph_Mouth_Speech_U" "/Game/Speech/CV_SpeechAnim.CV_SpeechAnim" 2.0 1.0 (`self.FacialAnimationDuration`) 0.99)))))

(event `ReceiveDestroyed_1`
  (`self.EndPlayFragments`))

(event `EnhancedInput|/Game/Input/IA_Jump`
  (params (ActionValue :type Boolean) (ElapsedSeconds :type "Float (double-precision)") (TriggeredSeconds :type "Float (double-precision)") (InputAction :type "InputAction Object Reference" :default "/Game/Input/IA_Jump.IA_Jump"))
  (:`Triggered`
    (`self.Jump`)
    ;[1 1 1] For physics Animation
    (`PrimitiveComponent.WakeAllRigidBodies` (`self.Mesh`) :!label _label)))

(event `EnhancedInput|/Game/Input/IA_Look`
  (params (ActionValue :type "Vector2D Structure") (ElapsedSeconds :type "Float (double-precision)") (TriggeredSeconds :type "Float (double-precision)") (InputAction :type "InputAction Object Reference" :default "/Game/Input/IA_Look.IA_Look"))
  (bind (_x _y) (`KismetMathLibrary.BreakVector2D` ActionValue))
  (:`Triggered`
    (`self.LookUpAtRate` _y)
    (`self.TurnAtRate` _x)
    (goto _label)))

(event `EnhancedInput|/Game/Input/IA_Move`
  (params (ActionValue :type "Vector2D Structure") (ElapsedSeconds :type "Float (double-precision)") (TriggeredSeconds :type "Float (double-precision)") (InputAction :type "InputAction Object Reference" :default "/Game/Input/IA_Move.IA_Move"))
  (bind (_x _y) (`KismetMathLibrary.BreakVector2D` ActionValue))
  (:`Triggered`
    (`self.MoveForward` _y)
    (`self.MoveRight` _x)
    (goto _label)))

(event `EnhancedInput|/Game/Input/IA_Continue_Skip_Dialogue`
  (params (ActionValue :type Boolean) (ElapsedSeconds :type "Float (double-precision)") (TriggeredSeconds :type "Float (double-precision)") (InputAction :type "InputAction Object Reference" :default "/Game/Input/IA_Continue_Skip_Dialogue.IA_Continue_Skip_Dialogue"))
  (:`Triggered`
    (bind _returnvalue (`JointSubsystem.GetAllJoints`))
    (for _array_element _returnvalue
      (`AbilitySystemBlueprintLibrary.SendGameplayEventToActor` _array_element (struct :`TagName` "JointNative.Input.SkipAndSelect")))))

(event `EnhancedInput|/Game/Input/IA_Run`
  (params (ActionValue :type Boolean) (ElapsedSeconds :type "Float (double-precision)") (TriggeredSeconds :type "Float (double-precision)") (InputAction :type "InputAction Object Reference" :default "/Game/Input/IA_Run.IA_Run"))
  (:`Triggered`
    (`self.AbilityInputPressed` (struct :`TagName` "JointPublicShowcase.Input.Run")))
  (:`Completed`
    (`self.AbilityInputReleased` (struct :`TagName` "JointPublicShowcase.Input.Run"))))

(event `EnhancedInput|/Game/Input/IA_Grab`
  (params (ActionValue :type Boolean) (ElapsedSeconds :type "Float (double-precision)") (TriggeredSeconds :type "Float (double-precision)") (InputAction :type "InputAction Object Reference" :default "/Game/Input/IA_Grab.IA_Grab"))
  (:`Triggered`
    (`self.AbilityInputPressed` (struct :`TagName` "JointPublicShowcase.Input.Grab")))
  (:`Completed`
    (`self.AbilityInputReleased` (struct :`TagName` "JointPublicShowcase.Input.Grab"))))

(event `Server_SetIsRunning`
  (params (bIsRunning :type Boolean))
  ;[1 1 1] Sorry I was a little out of time and didn't have time to implement GAS for this proj
  (set `self.bIsRunning` bIsRunning))

(fn `Death`
  (if (not (`self.IsDead`))
    (set `self.IsDead` true)
    (`self.Explode`)
    (`KismetSystemLibrary.K2_SetTimerDelegate` (`|CreateDelegate` :!event `K2_DestroyActor`) 3.0)))

(fn `Explode`
  (bind _returnvalue (`self.K2_GetActorLocation`))
  (bind _returnvalue_2 (`self.K2_GetActorLocation`))
  (`ActorComponent.Deactivate` (`self.CharacterMovement`))
  (`self.Set Physical Animations` true)
  (`PrimitiveComponent.SetSimulatePhysics` (`self.Mesh`) true)
  (`|ExecutionSequence`
    (:`then_0`
      (bind _outhits (`KismetSystemLibrary.SphereTraceMultiByProfile` :`Start` _returnvalue :`End` _returnvalue :`Radius` 50.0 :`ProfileName` "OverlapAll" :`bIgnoreSelf` false))
      (for _array_element _outhits
        (bind (_bblockinghit _binitialoverlap _time _distance _location _impactpoint _normal _impactnormal _physmat _hitactor _hitcomponent _hitbonename) (`GameplayStatics.BreakHitResult` _array_element))
        (bind _asskeletal_mesh_component (cast `SkeletalMeshComponent` _hitcomponent))
        (`PrimitiveComponent.AddImpulse` _asskeletal_mesh_component (`KismetMathLibrary.ClampVectorSize` (- (+ (`self.K2_GetActorLocation`) (* (`KismetMathLibrary.RandomUnitVector`) (5.0 5.0 5.0))) (`SceneComponent.GetSocketLocation` _asskeletal_mesh_component _hitbonename)) (`self.DeathExplosionForceMultiplier`) 5000.0) _hitbonename true)))
    (:`then_1`
      (`NiagaraFunctionLibrary.SpawnSystemAtLocation` "/Game/Particles/NS_DustExplosion.NS_DustExplosion" _returnvalue_2 (struct) (0.5 0.5 0.5))
      (`GameplayStatics.SpawnSoundAtLocation` "/Game/Sounds/Expression_ClearPop.Expression_ClearPop" _returnvalue_2 (struct) 1.0 1.0 0.0 null null))))

(fn `GetFragments`
  (returns (OutFragments :type "Array of CharacterFragment Object Reference"))
  (locals (NewLocalVar_0 :type "Array of CharacterFragment Object Reference"))
  (`|ExecutionSequence`
    (:`then_0`
      (`KismetArrayLibrary.Array_Clear` (`local.NewLocalVar_0`)))
    (:`then_1`
      (for _array_element (`self.Fragments`)
        (`KismetArrayLibrary.Array_Add` (`local.NewLocalVar_0`) (`.FragmentInstance` (break `CharacterFragmentElement` _array_element)))))
    (:`then_2`
      (return (`local.NewLocalVar_0`)))))

(fn `GetIsDead`
  (returns (NewParam :type Boolean))
  (return (`self.IsDead`)))

(fn `LinkAnimLayer`
  (params (InClass :type "AnimInstance Class Reference"))
  (`SkeletalMeshComponent.LinkAnimClassLayers` (`self.Mesh`) InClass))

(fn `OnRep_bIsRunning`
  (if (`self.bIsRunning`)
    (set `CharacterMovementComponent.MaxWalkSpeed` 2000.0 (`self.CharacterMovement`))
    (else
      (set `CharacterMovementComponent.MaxWalkSpeed` 500.0 (`self.CharacterMovement`)))))

(fn `Set Physical Animations`
  (params (bClear :type Boolean))
  (bind _physicalanimation (`self.PhysicalAnimation`))
  (bind _mesh (`self.Mesh`))
  (if bClear
    (`PhysicalAnimationComponent.SetStrengthMultiplyer` _physicalanimation 0.0)
    (`PhysicalAnimationComponent.SetSkeletalMeshComponent` _physicalanimation null)
    (else
      (`PhysicalAnimationComponent.SetStrengthMultiplyer` (`self.PhysicalAnimation`) 1.0)
      (`|ExecutionSequence`
        (:`then_0`
          (`PhysicalAnimationComponent.SetSkeletalMeshComponent` (`self.PhysicalAnimation`) (`self.Mesh`)))
        (:`then_1`
          (for _array_element (`self.Physical Animation Data`)
            (bind (_physdata _bonename _physicsblendweight) (break `/Game/Animations/AnimStruct_PhysicsAnimationBoneNameData` _array_element))
            (for _array_element_2 _bonename
              (`PhysicalAnimationComponent.ApplyPhysicalAnimationSettingsBelow` (`self.PhysicalAnimation`) _array_element_2 _physdata true)
              (`SkeletalMeshComponent.SetAllBodiesBelowSimulatePhysics` _mesh _array_element_2 true true)
              (`SkeletalMeshComponent.SetAllBodiesBelowPhysicsBlendWeight` _mesh _array_element_2 _physicsblendweight false true))))))))

(fn `StartTickTimer`
  (params (TickEvent :type Delegate))
  (bind _returnvalue (`KismetSystemLibrary.K2_SetTimerDelegate` TickEvent (`self.TickIntervalTime`) true))
  (set `self.TickTimer` _returnvalue))

(fn `Unexplode`
  (bind _mesh (`self.Mesh`))
  (`ActorComponent.Activate` (`self.CharacterMovement`) false)
  (`PrimitiveComponent.SetSimulatePhysics` _mesh false)
  (`self.Set Physical Animations` false)
  (`SceneComponent.K2_AttachToComponent` _mesh (`self.CapsuleComponent`) "None" "KeepWorld" "KeepWorld" "KeepWorld" true))

(fn `UserConstructionScript`)