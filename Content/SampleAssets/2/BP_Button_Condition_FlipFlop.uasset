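; BP_Button_Condition_FlipFlop is a button that toggles a boolean condition, IsActive, each time it is pressed.
; The server press event inverts IsActive and writes the new value to the StateValue text.
; Construction script and BeginPlay also refresh that text to show the starting state.
; Client press and both release events are empty, and this graph's only text update after BeginPlay runs in the server press event.
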(event `self.ReceiveBeginPlay`
  (`TextRenderComponent.K2_SetText` (`self.StateValue`) (`KismetTextLibrary.Conv_BoolToText` (`self.bIsActive`))))

(event `Server_OnPressed`
  (set `self.bIsActive` (not (`self.bIsActive`)))
  (`TextRenderComponent.K2_SetText` (`self.StateValue`) (`KismetTextLibrary.Conv_BoolToText` (`self.bIsActive`))))

(event `Client_OnPressed`)

(event `Server_OnReleased`)

(event `Client_OnReleased`)

(fn `UserConstructionScript`
  (`TextRenderComponent.K2_SetText` (`self.StateValue`) (`KismetTextLibrary.Conv_BoolToText` (`self.bIsActive`))))