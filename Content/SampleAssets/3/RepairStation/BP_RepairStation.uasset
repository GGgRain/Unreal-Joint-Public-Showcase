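; Repair station Blueprint that counts an exploded character's body parts inside its box and can revive that character.
; While open, a looping timer box-traces for unique bones of the target's mesh; box overlaps also trigger a count.
; It displays the current count and broadcasts when the highest count rises.
; Open/Close drive button animation, sound and light; separate functions unexplode and teleport the target or play the revive sequence.
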(event `self.ReceiveBeginPlay`
  (`self.Change Cosmetic Pressed` (`self.bOpened`))
  (`KismetSystemLibrary.K2_SetTimerDelegate` (delegate `Tick`) 0.2 true))

(event `Tick`
  (if (`self.bOpened`)
    (bind (_oldcount _newcount) (`self.Update Max Parts Count` :!label _label))
    (`|ExecutionSequence`
      (:`then_0`
        (if (< _oldcount _newcount)
          (`self.OnPartCountChanged` (`self.MaxPartsCount`))))
      (:`then_1`
        (`TextRenderComponent.K2_SetText` (`self.TextRender`) (`KismetTextLibrary.Conv_StringToText` (`KismetStringLibrary.Conv_IntToString` (`self.CurPartsCount`))))))))

(event `self.Box.OnComponentBeginOverlap`
  (params (OverlappedComponent :type "PrimitiveComponent Object Reference") (OtherActor :type "Actor Object Reference") (OtherComp :type "PrimitiveComponent Object Reference") (OtherBodyIndex :type Integer) (bFromSweep :type Boolean) (SweepResult :type "HitResult Structure (by ref)"))
  (goto _label))

(event `Open`
  (bind _output_get (set `self.bOpened` true))
  (`self.Change Cosmetic Pressed` _output_get))

(event `Close`
  (bind _output_get (set `self.bOpened` false))
  (`self.Change Cosmetic Pressed` _output_get))

(fn `Change Cosmetic Pressed`
  (params (bPressed :type Boolean))
  (bind _asabp_repair_station (cast `/Game/SampleAssets/3/RepairStation/ABP_RepairStation` (`SkeletalMeshComponent.GetAnimInstance` (`self.SkeletalMesh`))))
  (bind _output_get (set `/Game/SampleAssets/3/RepairStation/ABP_RepairStation.bPressed` bPressed _asabp_repair_station))
  (if _output_get
    (`ActorComponent.Activate` (`self.SC_Button_Press`) true)
    (`LightComponent.SetIntensity` (`self.RectLight`) 5000.0)
    (else
      (`ActorComponent.Activate` (`self.SC_Button_Release`) true)
      (`LightComponent.SetIntensity` (`self.RectLight`) 0.0))))

(fn `ReviveCharacter`
  (bind _output (`|ConvertAsset` (`self.Target Actor`)))
  (`/Game/Global/Characters/Pekorobo/BP_Character_Pekorobo.Unexplode` _output)
  (`self.K2_SetActorLocation` _output (`self.K2_GetActorLocation`) false true)
  (`self.K2_SetActorLocation` _output (`self.K2_GetActorLocation`) false true))

(fn `ReviveCharacterAnimation`
  (bind _outactor (`LevelSequencePlayer.CreateLevelSequencePlayer` "/Game/SampleAssets/3/RepairStation/animations/LS_Revive.LS_Revive"))
  (`MovieSceneSequencePlayer.Play` (`LevelSequenceActor.SequencePlayer` _outactor)))

(fn `Update Max Parts Count`
  (returns (OldCount :type Integer) (NewCount :type Integer))
  (locals (CachedOldCount :type Integer :default 0) (Temp :type Integer) (KnownBones :type "Set of Name"))
  (bind (_origin _boxextent) (`KismetSystemLibrary.GetComponentBounds` (`self.Box`)))
  (set `local.CachedOldCount` (`self.MaxPartsCount`))
  (bind _outhits (`KismetSystemLibrary.BoxTraceMultiByProfile` _origin _origin _boxextent (struct) "OverlapAllNoPawn"))
  (for _array_element _outhits
    (bind (_bblockinghit _binitialoverlap _time _distance _location _impactpoint _normal _impactnormal _physmat _hitactor _hitcomponent _hitbonename) (`GameplayStatics.BreakHitResult` _array_element))
    (if (== (`Character.Mesh` (`|ConvertAsset` (`self.Target Actor`))) _hitcomponent)
      (if (not (`BlueprintSetLibrary.Set_Contains` (`local.KnownBones`) _hitbonename))
        (`/Engine/EditorBlueprintResources/StandardMacros.IncrementInt` (`local.Temp`)
          (:`  `
            (`BlueprintSetLibrary.Set_Add` (`local.KnownBones`) _hitbonename))))))
  (set `self.CurPartsCount` (`local.Temp`))
  (bind _output_get (set `self.MaxPartsCount` (`KismetMathLibrary.Max` (`self.MaxPartsCount`) (`local.Temp`))))
  (return (`local.CachedOldCount`) _output_get))

(fn `UserConstructionScript`)