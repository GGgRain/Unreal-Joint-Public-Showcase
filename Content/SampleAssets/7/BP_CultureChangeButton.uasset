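; BP_CultureChangeButton is a pressable button that switches the game's culture for localization.
; Both server and client press events call SetCurrentCulture with the configured Culture, while release events do nothing.
; The construction script labels Display0 with "Change Culture" and the culture code unless custom display text is enabled.
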(event `Server_OnPressed`
  (`KismetInternationalizationLibrary.SetCurrentCulture` (`self.Culture`) :!label _label))

(event `Client_OnPressed`
  (goto _label))

(event `Server_OnReleased`)

(event `Client_OnReleased`)

(fn `UserConstructionScript`
  (if (not (`self.bUseCustomDisplayText`))
    (`TextRenderComponent.K2_SetText` (`self.Display_0`) (`KismetTextLibrary.Conv_StringToText` (`KismetStringLibrary.Concat_StrStr` "Change Culture" ":" (`self.Culture`))))))