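; A sample trigger button that plays a Joint dialogue using characters from a linked spawn button as participants.
; On a press, server-authority events optionally end the last joint actor, then create and start a new one from the assigned joint manager.
; Before starting, it maps participant fragments by tag and binds each spawned character's dialogue participant component through an index-to-tag list.
; The construction script labels the button with the manager's name unless custom text is used.
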(event `self.Server_OnPressed`
  (`|ExecutionSequence`
    (:`then_0`
      (`self.Server_EndDialogue`))
    (:`then_1`
      (`self.Server_StartDialogue`))))

(event `Server_EndDialogue`
  (`/Engine/EditorBlueprintResources/ActorMacros.Switch Has Authority`
    (:`Authority`
      (if (`self.bDestroyOldJointActorWhenPressed`)
        (`/Engine/EditorBlueprintResources/StandardMacros.IsValid` (`self.LastlyPlayedJointActor`)
          (:`Is Valid`
            (`JointActor.EndJoint` (`self.LastlyPlayedJointActor`))
            (set `self.LastlyPlayedJointActor` null)))))))

(event `Server_StartDialogue`
  (`/Engine/EditorBlueprintResources/ActorMacros.Switch Has Authority`
    (:`Authority`
      (bind _returnvalue (`JointSubsystem.CreateJoint` (`self.JointManagerToPlay`)))
      (bind _output_get (set `self.LastlyPlayedJointActor` _returnvalue))
      (`|ExecutionSequence`
        (:`then_0`
          (`self.Feed Overriden Participants` _output_get))
        (:`then_1`
          (`JointActor.StartJoint` _output_get))))))

(fn `Feed Overriden Participants`
  (params (`Joint Actor` :type "JointActor Object Reference"))
  (locals (CachedParticipants :type "Map of GameplayTag Structure to DF_Participant Object Reference") (TagsForIndices :type "Array of GameplayTag Structure"))
  (`|ExecutionSequence`
    (:`then_0`
      (for _array_element (`JointManager.FindManagerFragmentsByClassOnLowerHierarchy` (`JointActor.GetJointManager` `Joint Actor`) "/Script/JointNative.DF_Participant")
        (`BlueprintMapLibrary.Map_Add` (`local.CachedParticipants`) (`DF_Participant.ParticipantTag` _array_element) _array_element)))
    (:`then_1`
      (for (_array_element_2 _array_index) (`/Game/SampleAssets/5/BP_CharacterSpawnButton.SpawnedCharacters` (`|ConvertAsset` (`self.CharacterSpawnButton`)))
        (bind (_value _returnvalue) (`BlueprintMapLibrary.Map_Find` (`local.CachedParticipants`) (`|GetArrayItem` (`local.TagsForIndices`) _array_index)))
        (if _returnvalue
          (set `DF_Participant.ParticipantComponentInstance` (`self.GetComponentByClass` _array_element_2 "/Script/JointNative.DialogueParticipantComponent") _value))))))

(fn `UserConstructionScript`
  (if (not (`self.bUseCustomDisplayText`))
    (`TextRenderComponent.K2_SetText` (`self.Display`) (`KismetTextLibrary.Conv_StringToText` (`KismetStringLibrary.Concat_StrStr` "Play Dialogue" ":" (`KismetSystemLibrary.GetObjectName` (`self.JointManagerToPlay`)))))))