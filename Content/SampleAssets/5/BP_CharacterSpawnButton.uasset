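; Pressable button Blueprint that spawns half-scale BP_Character_Pekorobo characters, handled in its ServeronPressed event.
; Each press places one at a random XY point and yaw within the SpawnBound component, with a dust Niagara effect and pop sound.
; It tracks spawns in SpawnedCharacters, calling Death on the oldest before spawning to cap the list at nine.
; The construction script's Display label update is disabled by a constant condition.
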(event `self.Server_OnPressed`
  (`|ExecutionSequence`
    (:`then_0`
      (if (>= (`KismetArrayLibrary.Array_Length` (`self.SpawnedCharacters`)) 9)
        (`/Game/Global/Characters/Pekorobo/BP_Character_Pekorobo.Death` (`|GetArrayItem` (`self.SpawnedCharacters`)))
        (`KismetArrayLibrary.Array_Remove` (`self.SpawnedCharacters`))))
    (:`then_1`
      (bind _returnvalue (`|SpawnActorFromClass` "/Game/Global/Characters/Pekorobo/BP_Character_Pekorobo.BP_Character_Pekorobo_C" (`self.GetRandomSpawnTransform`) "AdjustIfPossibleButAlwaysSpawn" "OverrideRootScale" null null))
      (bind _returnvalue_2 (`self.K2_GetActorLocation` _returnvalue))
      (`NiagaraFunctionLibrary.SpawnSystemAtLocation` "/Game/Global/Particles/NS_DustExplosion.NS_DustExplosion" _returnvalue_2 (struct) (0.5 0.5 0.5))
      (`GameplayStatics.SpawnSoundAtLocation` "/Game/Global/Sounds/Expression_ClearPop.Expression_ClearPop" _returnvalue_2 (struct) 1.0 1.0 0.0 "/Game/Global/PhysicsSound/Default/SA_Master.SA_Master" null)
      (`KismetArrayLibrary.Array_Add` (`self.SpawnedCharacters`) _returnvalue))))

(fn `GetRandomSpawnTransform`
  (returns (ReturnValue :type "Transform Structure"))
  (bind (_origin _boxextent) (`KismetSystemLibrary.GetComponentBounds` (`self.SpawnBound`)))
  (bind (_x _y) (`KismetMathLibrary.BreakVector3f` _boxextent))
  (return (`KismetMathLibrary.MakeTransform` (+ _origin (`KismetMathLibrary.MakeVector` (`KismetMathLibrary.RandomFloatInRange` (* _x -1.0) _x) (`KismetMathLibrary.RandomFloatInRange` (* _y -1.0) _y))) (`KismetMathLibrary.MakeRotator` 0.0 0.0 (`KismetMathLibrary.RandomFloatInRange` -180.0 180.0)) (0.5 0.5 0.5))))

(fn `UserConstructionScript`
  (if (not true)
    (`TextRenderComponent.K2_SetText` (`self.Display`) (`KismetTextLibrary.Conv_StringToText` (`KismetStringLibrary.Concat_StrStr` "Play Dialogue" ":" (`KismetSystemLibrary.GetObjectName` null))))))