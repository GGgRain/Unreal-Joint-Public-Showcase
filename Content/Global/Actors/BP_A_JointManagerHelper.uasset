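; An in-level helper actor that opens the referenced JointManager asset in the editor when a player-controlled Character walks into its Box trigger.
; The construction script labels its TextRender with the asset's name, trimmed at the first dot, unless UseCustomText is set.
; A fast looping timer started on BeginPlay accumulates elapsed time into a sine that bobs the StaticMesh gently up and down, without using Tick.
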(event `self.ReceiveBeginPlay`
  (bind _returnvalue (`KismetSystemLibrary.K2_SetTimerDelegate` (delegate `Timer`) 0.01 true))
  (set `self.TimerHandle` _returnvalue))

(event `Timer`
  (set `self.FloatingVal` (+ (`self.FloatingVal`) (`KismetSystemLibrary.K2_GetTimerElapsedTimeHandle` (`self.TimerHandle`))))
  (`SceneComponent.K2_SetRelativeLocation` (`self.StaticMesh`) (`KismetMathLibrary.MakeVector` 0.0 0.0 (* (`KismetMathLibrary.Sin` (`self.FloatingVal`)) 3.0)) false false))

(event `self.Box.OnComponentBeginOverlap`
  (params (OverlappedComponent :type "PrimitiveComponent Object Reference") (OtherActor :type "Actor Object Reference") (OtherComp :type "PrimitiveComponent Object Reference") (OtherBodyIndex :type Integer) (bFromSweep :type Boolean) (SweepResult :type "HitResult Structure (by ref)"))
  (bind _ascharacter (cast `Character` OtherActor))
  (cast `PlayerController` (`Pawn.GetController` _ascharacter))
  (`BasicStuffBPFL.OpenEditorForAsset` (`|ConvertAsset` (`self.JointManager`))))

(fn `UserConstructionScript`
  (if (not (`self.bUseCustomText`))
    (`TextRenderComponent.K2_SetText` (`self.TextRender`) (`KismetTextLibrary.Conv_StringToText` (`KismetStringLibrary.Split` (`KismetSystemLibrary.Conv_SoftObjectReferenceToString` (`self.JointManager`)) ".")))))