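; World button that plays a dialogue Joint asset when pressed, labelled with the asset's name unless custom text is used.
; A press either toggles the dialogue or restarts it, with ending the previous Joint actor gated by a flag.
; On authority, it creates the Joint and binds participant components from an override map of target actors or player pawns.
; Outside standalone, it delays starting briefly so participants can replicate.
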(event `self.Server_OnPressed`
  (if (`self.bUseFlipFlop`)
    (`/Engine/EditorBlueprintResources/StandardMacros.IsValid` (`self.LastlyPlayedJointActor`)
      (:`Is Valid`
        (`self.Server_EndDialogue`))
      (:`Is Not Valid`
        (`self.Server_StartDialogue`)))
    (else
      (`|ExecutionSequence`
        (:`then_0`
          (`self.Server_EndDialogue`))
        (:`then_1`
          (`self.Server_StartDialogue`))))))

(event `self.Server_OnReleased`)

(event `Server_EndDialogue`
  (`/Engine/EditorBlueprintResources/ActorMacros.Switch Has Authority`
    (:`Authority`
      (if (`self.bDestroyOldJointActorWhenPressed`)
        (`/Engine/EditorBlueprintResources/StandardMacros.IsValid` (`self.LastlyPlayedJointActor`)
          (:`Is Valid`
            (`JointActor.EndJoint` (`self.LastlyPlayedJointActor`))
            (set `self.LastlyPlayedJointActor` null)))))))

(event `Server_StartDialogue`
  (`/Engine/EditorBlueprintResources/ActorMacros.Switch Has Authority`
    (:`Authority`
      (bind _returnvalue (`JointSubsystem.CreateJoint` (`self.JointManagerToPlay`)))
      (bind _output_get (set `self.LastlyPlayedJointActor` _returnvalue))
      (`|ExecutionSequence`
        (:`then_0`
          (`self.Feed Overriden Participants` _output_get))
        (:`then_1`
          ;[1 1 1] Make it wait the replication for the participant
          (if (not (`KismetSystemLibrary.IsStandalone`))
            (`KismetSystemLibrary.Delay` 0.2))
          (`JointActor.StartJoint` (`self.LastlyPlayedJointActor`)))))))

(fn `Feed Overriden Participants`
  (params (`Joint Actor` :type "JointActor Object Reference"))
  (for _array_element (`JointManager.FindManagerFragmentsByClassOnLowerHierarchy` (`JointActor.GetJointManager` `Joint Actor`) "/Script/JointNative.DF_Participant")
    (bind (_value _returnvalue) (`BlueprintMapLibrary.Map_Find` (`self.ParticipantOverrideMap`) (`DF_Participant.ParticipantTag` _array_element)))
    (bind (_targetactor _buseplayercontrollercontrolledpawn _playercontrollerindex) (break `/Game/Global/Actors/Button/ST_ButtonParticipantOverrideSettings` _value))
    (if _buseplayercontrollercontrolledpawn
      (set `DF_Participant.ParticipantComponentInstance` (`self.GetComponentByClass` (`Controller.K2_GetPawn` (`GameplayStatics.GetPlayerController` _playercontrollerindex)) "/Script/JointNative.DialogueParticipantComponent") _array_element)
      (elif _returnvalue
        (set `DF_Participant.ParticipantComponentInstance` (`self.GetComponentByClass` (`|ConvertAsset` _targetactor) "/Script/JointNative.DialogueParticipantComponent") _array_element)))))

(fn `OnRep_LastlyPlayedJointActor`)

(fn `UserConstructionScript`
  (if (not (`self.bUseCustomDisplayText`))
    (`TextRenderComponent.K2_SetText` (`self.Display`) (`KismetTextLibrary.Conv_StringToText` (`KismetStringLibrary.Concat_StrStr` "Play Dialogue" ":" (`KismetSystemLibrary.GetObjectName` (`self.JointManagerToPlay`)))))))