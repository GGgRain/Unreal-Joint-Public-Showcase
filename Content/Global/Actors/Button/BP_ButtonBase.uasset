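; Base button actor that is pressed and released by overlaps on its box, optionally limited to player-controlled characters.
; Overlaps drive the button's animation Blueprint and press/release sounds, then call empty server or client hook events based on authority.
; Presses are gated by a timer-handle cooldown and a replay check, and only the authority starts the cooldown.
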(event `Server_OnPressed`)

(event `Client_OnPressed`)

(event `Server_OnReleased`)

(event `Client_OnReleased`)

(event `self.Box.OnComponentBeginOverlap`
  (params (OverlappedComponent :type "PrimitiveComponent Object Reference") (OtherActor :type "Actor Object Reference") (OtherComp :type "PrimitiveComponent Object Reference") (OtherBodyIndex :type Integer) (bFromSweep :type Boolean) (SweepResult :type "HitResult Structure (by ref)"))
  (if (`self.CanInteract` OtherActor)
    (if (`self.CanBePlayed`)
      (`|ExecutionSequence`
        (:`then_0`
          (`self.Change Cosmetic Pressed` true))
        (:`then_1`
          (bind _ascharacter (cast `Character` OtherActor))
          (if (`self.HasAuthority` _ascharacter)
            (if (`self.IsOnCooldown`)
              (`self.Client_OnPressed`)
              (else
                (`self.SetCooldown`)
                (`self.Server_OnPressed`)))))))))

(event `OnCooldownExpired`
  (`KismetSystemLibrary.K2_ClearAndInvalidateTimerHandle` (`self.Timer`)))

(event `self.Box.OnComponentEndOverlap`
  (params (OverlappedComponent :type "PrimitiveComponent Object Reference") (OtherActor :type "Actor Object Reference") (OtherComp :type "PrimitiveComponent Object Reference") (OtherBodyIndex :type Integer))
  (if (`self.CanInteract` OtherActor)
    (`|ExecutionSequence`
      (:`then_0`
        (`self.Change Cosmetic Pressed` false))
      (:`then_1`
        (bind _ascharacter (cast `Character` OtherActor))
        (if (`self.HasAuthority` _ascharacter)
          (`self.Server_OnReleased`)
          (else
            (`self.Client_OnReleased`)))))))

(fn `CanBePlayed`
  (returns (CanBePlayed :type Boolean))
  (if (`self.IsOnCooldown`)
    (return false)
    (elif (`self.bEverPlayed`)
      (if (`self.bAllowPlayingAgain`)
        (return true)
        (else
          (return false)))
      (else
        (return true)))))

(fn `CanInteract`
  (params (Object :type "Object Object Reference"))
  (returns (ReturnValue :type Boolean))
  (if (`self.bInteractWithPlayersOnly`)
    (`|ExecutionSequence`
      (:`then_0`
        (bind _ascharacter (cast `Character` Object))
        (cast `PlayerController` (`Pawn.GetController` _ascharacter))
        (return true))
      (:`then_1`
        (return false)))
    (else
      (return true))))

(fn `Change Cosmetic Pressed`
  (params (bPressed :type Boolean))
  (bind _asabp_button (cast `/Game/Global/Actors/Button/ABP_Button` (`SkeletalMeshComponent.GetAnimInstance` (`self.SkeletalMesh`))))
  (set `/Game/Global/Actors/Button/ABP_Button.bPressed` bPressed _asabp_button)
  (if bPressed
    (`ActorComponent.Activate` (`self.SC_Button_Press`) true)
    (else
      (`ActorComponent.Activate` (`self.SC_Button_Release`) true))))

(fn `IsOnCooldown`
  (returns (ReturnValue :type Boolean))
  (return (`KismetSystemLibrary.K2_IsValidTimerHandle` (`self.Timer`))))

(fn `SetCooldown`
  (if (not (`KismetSystemLibrary.K2_IsTimerActiveHandle` (`self.Timer`)))
    (bind _returnvalue (`KismetSystemLibrary.K2_SetTimerDelegate` (`|CreateDelegate` :!event `OnCooldownExpired`) (`self.Cooldown`)))
    (set `self.Timer` _returnvalue)))

(fn `UserConstructionScript`)