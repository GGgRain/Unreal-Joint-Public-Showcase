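; BP_ScreenshotDisplayer is an actor that shows a chosen image on a plane mesh in the level.
; The construction script synchronously loads the soft-referenced image and material, then applies a dynamic material instance to the plane.
; It scales the plane by the image's pixel size times ImageScale to match its aspect ratio and feeds the image into a named texture parameter.
; The event graph holds no logic.
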(fn `UserConstructionScript`
  (`|ExecutionSequence`
    (:`then_0`
      (`KismetSystemLibrary.LoadAsset_Blocking` (`self.ImageToShow`))
      (`KismetSystemLibrary.LoadAsset_Blocking` (`self.MaterialToUse`))
      (bind _returnvalue (`KismetMaterialLibrary.CreateDynamicMaterialInstance` (`|ConvertAsset` (`self.MaterialToUse`))))
      (set `self.DMI` _returnvalue)
      (`PrimitiveComponent.SetMaterial` (`self.Plane`) 0 _returnvalue))
    (:`then_1`
      (`SceneComponent.SetWorldScale3D` (`self.Plane`) (`KismetMathLibrary.MakeVector` (* (`self.ImageScale`) (`KismetMathLibrary.Conv_IntToDouble` (`Texture2D.Blueprint_GetSizeX` (`|ConvertAsset` (`self.ImageToShow`))))) (* (`self.ImageScale`) (`KismetMathLibrary.Conv_IntToDouble` (`Texture2D.Blueprint_GetSizeY` (`|ConvertAsset` (`self.ImageToShow`))))) 1.0))
      (`MaterialInstanceDynamic.SetTextureParameterValue` (`self.DMI`) (`self.ImageTextureParameterName`) (`|ConvertAsset` (`self.ImageToShow`))))))