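; Speech synthesizer component that voices dialogue text as per-character syllable sounds for conversation participants.
; Each PlaySpeechFor call transliterates the current character to Latin, with a looping timer spreading multi-letter results across the sustain duration.
; Letters, with "sh" and "th" merged, select sounds through an integer parameter on a spawned audio component.
; Pitch and volume vary randomly and with distance to upcoming "!" or "?" marks.
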(event `self.ReceiveBeginPlay`
  (`self.InitSpeechAudioComponent`)
  (`self.InitTransliterator`))

(event `self.ReceiveEndPlay`
  (params (EndPlayReason :type "EEndPlayReason Enum" :default "Destroyed"))
  (`self.DiscardSpeechAudioComponent`))

(event `Play Speech For`
  (params (InstigatorParticipant :type "DialogueParticipantComponent Object Reference") (FromParticipants :type "Array of DialogueParticipantComponent Object Reference") (ToParticipants :type "Array of DialogueParticipantComponent Object Reference") (`Whole String` :type String) (CurrentIndex :type Integer))
  (`self.InitPlaySpeech` InstigatorParticipant FromParticipants ToParticipants `Whole String` CurrentIndex (delegate `PlaySpeechForCurrentLetter`)))

(event `PlaySpeechForCurrentLetter`
  (`self.PlaySpeechInternal`))

(fn `CacheSoundGroup`
  (params (SourceString :type String) (Start :type Integer))
  (bind (_isinbound _returnvalue) (`self.MidCheck` SourceString Start))
  (bind (_isinbound_2 _returnvalue_2) (`self.MidCheck` SourceString (+ Start 1)))
  (set `self.CachedWholeString` SourceString)
  (set `self.CachedCurrentIndex` Start)
  (set `self.PreviousSoundGroup` (`self.CurrentSoundGroup`))
  (if (`KismetStringLibrary.EqualEqual_StrStr` (`self.NextSoundGroup`))
    (if _isinbound
      (set `self.CurrentSoundGroup` (`ICUTransliteratorWrapper.TransliterateString` (`self.Transliterator`) _returnvalue)))
    (else
      (set `self.CurrentSoundGroup` (`self.NextSoundGroup`))))
  (if _isinbound_2
    (bind _output_get (set `self.NextSoundGroup` (`ICUTransliteratorWrapper.TransliterateString` (`self.Transliterator`) _returnvalue_2)))
    (return)))

(fn `Calculate Additive Pitch Volume From with settings`
  (params (Distance :type Integer) (`Distance Threshold` :type Integer) (`b Should Use Linear Curve Influence` :type Boolean) (`Influence Additive Pitch` :type "Float (double-precision)") (`Influence Additive Volume` :type "Float (double-precision)"))
  (returns (`Out Additive Pitch` :type "Float (double-precision)") (`Out Additive Volume` :type "Float (double-precision)"))
  (bind _returnvalue (/ (`KismetMathLibrary.Conv_IntToDouble` Distance) (`KismetMathLibrary.Conv_IntToDouble` `Distance Threshold`)))
  (if (and (<= Distance `Distance Threshold`) (!= Distance -1))
    (if `b Should Use Linear Curve Influence`
      (return (* _returnvalue `Influence Additive Pitch`) (* _returnvalue `Influence Additive Volume`))
      (else
        (return `Influence Additive Pitch` `Influence Additive Volume`)))
    (else
      (return 0.0 0.0))))

(fn `CheckExclamationMarkDistance`
  (returns (Distance :type Integer))
  (bind _returnvalue (`KismetStringLibrary.FindSubstring` (`self.CachedWholeString`) "!" false false (`self.CachedCurrentIndex`)))
  (if (!= _returnvalue -1)
    (return (`KismetMathLibrary.Abs_Int` (- _returnvalue (`self.CachedCurrentIndex`))))
    (else
      (return -1))))

(fn `CheckQuestionMarkDistance`
  (returns (Distance :type Integer))
  (bind _returnvalue (`KismetStringLibrary.FindSubstring` (`self.CachedWholeString`) "?" false false (`self.CachedCurrentIndex`)))
  (if (!= _returnvalue -1)
    (return (`KismetMathLibrary.Abs_Int` (- _returnvalue (`self.CachedCurrentIndex`))))
    (else
      (return -1))))

(fn `CheckSh`
  (returns (ReturnValue :type Boolean))
  (bind _returnvalue (`self.GetPreviousSyllable`))
  (bind (_returnvalue_2 _isinbound) (`self.GetNextSyllable`))
  (bind (_returnvalue_3 _isinbound_2) (`self.GetCurrentSyllable`))
  (return (and (not (or (`KismetStringLibrary.EqualEqual_StrStr` _returnvalue " ") (`KismetStringLibrary.EqualEqual_StrStr` _returnvalue "?") (`KismetStringLibrary.EqualEqual_StrStr` _returnvalue "!"))) (and (and (== _returnvalue_3 "s") (== _returnvalue_2 "h")) (and _isinbound_2 _isinbound)))))

(fn `CheckShouldSlience`
  (returns (ReturnValue :type Boolean))
  (bind (_returnvalue _isinbound) (`self.GetCurrentSyllable`))
  (bind _returnvalue_2 (`self.GetCurrentSyllable`))
  (bind (_returnvalue_3 _isinbound_2) (`self.GetPreviousSyllable`))
  (bind (_returnvalue_4 _isinbound_3) (`self.GetCurrentSyllable`))
  (bind (_returnvalue_5 _isinbound_4) (`self.GetPreviousSyllable`))
  (return (or (and (and (== _returnvalue_3 "s") (== _returnvalue "h")) (and _isinbound_2 _isinbound)) (and (and (== _returnvalue_5 "t") (== _returnvalue_4 "h")) (and _isinbound_4 _isinbound_3)) (or (== _returnvalue_2 " ") (== _returnvalue_2 "?") (== _returnvalue_2 "!")))))

(fn `CheckTh`
  (returns (ReturnValue :type Boolean))
  (bind _returnvalue (`self.GetPreviousSyllable`))
  (bind (_returnvalue_2 _isinbound) (`self.GetNextSyllable`))
  (bind (_returnvalue_3 _isinbound_2) (`self.GetCurrentSyllable`))
  (return (and (not (or (`KismetStringLibrary.EqualEqual_StrStr` _returnvalue " ") (`KismetStringLibrary.EqualEqual_StrStr` _returnvalue "?") (`KismetStringLibrary.EqualEqual_StrStr` _returnvalue "!"))) (and (and (== _returnvalue_3 "t") (== _returnvalue_2 "h")) (and _isinbound_2 _isinbound)))))

(fn `DiscardSpeechAudioComponent`
  (bind _speechaudiocomponent (`self.SpeechAudioComponent`))
  (`/Engine/EditorBlueprintResources/StandardMacros.IsValid` _speechaudiocomponent
    (:`Is Valid`
      (`self.K2_DestroyComponent` _speechaudiocomponent)
      (set `self.SpeechAudioComponent` null))))

(fn `GetCurrentSyllable`
  (returns (ReturnValue :type String) (IsInBound :type Boolean))
  (bind _currentgroupiiterationcount (`self.CurrentGroupIIterationCount`))
  (bind _currentsoundgroup (`self.CurrentSoundGroup`))
  (if (< _currentgroupiiterationcount (`KismetStringLibrary.Len` _currentsoundgroup))
    (return (`KismetStringLibrary.Mid` _currentsoundgroup _currentgroupiiterationcount 1) true)
    (else
      (return "null" false))))

(fn `GetNextSyllable`
  (returns (ReturnValue :type String) (IsInBound :type Boolean))
  (locals (OutString :type String))
  (if (== (`self.CurrentGroupIIterationCount`) (- (`KismetStringLibrary.Len` (`self.CurrentSoundGroup`)) 1))
    (set `local.OutString` (`KismetStringLibrary.Mid` (`self.NextSoundGroup`) 0 1))
    (else
      (set `local.OutString` (`KismetStringLibrary.Mid` (`self.CurrentSoundGroup`) (+ (`self.CurrentGroupIIterationCount`) 1) 1))))
  (if true
    (return (`local.OutString`) true)
    (else
      (return "null" false))))

(fn `GetPreviousSyllable`
  (returns (ReturnValue :type String) (IsInBound :type Boolean))
  (locals (OutString :type String))
  (bind _previoussoundgroup (`self.PreviousSoundGroup`))
  (if (== (`self.CurrentGroupIIterationCount`) 0)
    (set `local.OutString` (`KismetStringLibrary.Mid` _previoussoundgroup (- (`KismetStringLibrary.Len` _previoussoundgroup) 1) 1))
    (else
      (set `local.OutString` (`KismetStringLibrary.Mid` (`self.CurrentSoundGroup`) (+ (`self.CurrentGroupIIterationCount`) -1) 1))))
  (if true
    (return (`local.OutString`) true)
    (else
      (return "null" false))))

(fn `GetSyllableToPlay`
  (returns (`Out Syllable` :type Name))
  (locals (FinalSyllable :type Name :default "sh"))
  (if (`self.CheckTh`)
    (set `local.FinalSyllable` "th")
    (return (`local.FinalSyllable`))
    (elif (`self.CheckSh`)
      (set `local.FinalSyllable` "sh")
      (return (`local.FinalSyllable`))
      (elif (not (`self.CheckShouldSlience`))
        (set `local.FinalSyllable` (`KismetStringLibrary.Conv_StringToName` (`self.GetCurrentSyllable`)))
        (return (`local.FinalSyllable`))))))

(fn `InitPlaySpeech`
  (params (InstigatorParticipant :type "DialogueParticipantComponent Object Reference") (FromParticipants :type "Array of DialogueParticipantComponent Object Reference") (ToParticipants :type "Array of DialogueParticipantComponent Object Reference") (WholeStr :type String) (CurrentIndex :type Integer) (Delegate :type Delegate))
  (bind _returnvalue (`KismetStringLibrary.Len` (`self.CurrentSoundGroup`)))
  (`|ExecutionSequence`
    (:`then_0`
      (set `self.Instigator Participant` InstigatorParticipant)
      (set `self.From Participants` FromParticipants)
      (set `self.To Participants` ToParticipants))
    (:`then_1`
      (`self.CacheSoundGroup` WholeStr CurrentIndex)
      (set `self.CurrentGroupIIterationCount` 0)
      (set `self.CurrentGroupIIterationMaxCount` _returnvalue)
      (`self.PlaySpeechForCurrentLetter`)
      (if (>= _returnvalue 2)
        (bind _returnvalue_2 (`KismetSystemLibrary.K2_SetTimerDelegate` Delegate (/ (`self.SoundSustainDuration`) (`KismetMathLibrary.Conv_IntToDouble` _returnvalue)) true))
        (set `self.SoundGroupPlaybackTimer` _returnvalue_2)))))

(fn `InitSpeechAudioComponent`
  (bind _returnvalue (`|AddComponentByClass` (`self.GetOwner`) "/Script/Engine.AudioComponent" false (`self.GetRelativeTransform`)))
  (set `AudioComponent.AttenuationSettings` (`self.Attenuation Settings`) _returnvalue)
  (bind _output_get (set `self.SpeechAudioComponent` _returnvalue))
  (`AudioComponent.SetSound` _output_get (`self.SyllableSoundSet`)))

(fn `InitTransliterator`
  (set `self.Transliterator` (`JointNativeFunctionLibrary.CreateTransliterator` "Any-Latin")))

(fn `Interface_ProvideParticipantTagContainer`
  (returns (`Participant Tag Container` :type "GameplayTagContainer Structure"))
  (return (`self.ParticipantTag`)))

(fn `MidCheck`
  (params (`Source String` :type String) (Index :type Integer))
  (returns (IsInBound :type Boolean) (ReturnValue :type String))
  (if (< Index (`KismetStringLibrary.Len` `Source String`))
    (return true (`KismetStringLibrary.Mid` `Source String` Index 1))
    (else
      (return false "null"))))

(fn `PlaySpeechInternal`
  (locals (FinalSyllable :type Name))
  (bind (_value _returnvalue) (`BlueprintMapLibrary.Map_Find` (`self.Syllables`) (`local.FinalSyllable`)))
  (`|ExecutionSequence`
    (:`then_0`
      (bind _out_syllable (`self.GetSyllableToPlay`))
      (bind _output_get (set `local.FinalSyllable` _out_syllable))
      (`self.OnSoundPlayed` _output_get))
    (:`then_1`
      (`self.Update Pitch And Volume with Marks`))
    (:`then_2`
      ;[1 1 1] Play Actual sound for the final syllable
      (if _returnvalue
        (`AudioComponent.SetIntParameter` (`self.SpeechAudioComponent`) (`self.SpeechSwitchParameterName`) _value)
        (`AudioComponent.Play` (`self.SpeechAudioComponent`) 0.0))
      (set `self.CurrentGroupIIterationCount` (+ (`self.CurrentGroupIIterationCount`) 1))
      (if (>= (`self.CurrentGroupIIterationCount`) (`self.CurrentGroupIIterationMaxCount`))
        (`KismetSystemLibrary.K2_ClearAndInvalidateTimerHandle` (`self.SoundGroupPlaybackTimer`))))))

(fn `Update Pitch And Volume with Marks`
  (bind (_out_additive_pitch _out_additive_volume) (`self.Calculate Additive Pitch Volume From with settings` (`self.CheckQuestionMarkDistance`) (`self.Exclamation Influence Distance`) true (`self.Question Influence Additive Pitch`) (`self.Question Influence Additive Volume`)))
  (bind (_out_additive_pitch_2 _out_additive_volume_2) (`self.Calculate Additive Pitch Volume From with settings` (`self.CheckExclamationMarkDistance`) (`self.Exclamation Influence Distance`) true (`self.Exclamation Influence Additive Pitch`) (`self.Exclamation Influence Additive Volume`)))
  (`|ExecutionSequence`
    (:`then_0`
      ;[1 1 1] Calculate the additive pitch and volumes.
      (set `self.AdditivePitch` (`KismetMathLibrary.FMax` _out_additive_pitch_2 _out_additive_pitch))
      (set `self.AdditiveVolume` (`KismetMathLibrary.FMax` _out_additive_volume_2 _out_additive_volume)))
    (:`then_1`
      ;[1 1 1] Apply it to the component
      (`AudioComponent.SetPitchMultiplier` (`self.SpeechAudioComponent`) (+ (`self.BasePitch`) (`self.AdditivePitch`) (* (* (- (`KismetMathLibrary.RandomFloat`) 0.5) 2.0) (`self.RandomPitch`))))
      (`AudioComponent.SetVolumeMultiplier` (`self.SpeechAudioComponent`) (+ (`self.BaseVolume`) (`self.AdditiveVolume`) (* (* (- (`KismetMathLibrary.RandomFloat`) 0.5) 2.0) (`self.RandomVolume`)))))))