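; Overlap-triggered button actor that spawns BP_Character_Pekorobo characters, with a dust effect and pop sound.
; Each spawn lands at a random point and yaw within the Box1 bounds at half scale, and the oldest character is killed to cap the population at nine.
; A timer handle gates retriggering during cooldown.
; Button feedback goes through the ABP_Button Pressed flag and press/release components, though both calls pass false.
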(event `self.Box.OnComponentBeginOverlap`
  (params (OverlappedComponent :type "PrimitiveComponent Object Reference") (OtherActor :type "Actor Object Reference") (OtherComp :type "PrimitiveComponent Object Reference") (OtherBodyIndex :type Integer) (bFromSweep :type Boolean) (SweepResult :type "HitResult Structure (by ref)"))
  (if (not (`self.IsCooldownOn`))
    (`self.SetCooldown`)
    (`self.Change Cosmetic Pressed` false)
    (`|ExecutionSequence`
      (:`then_0`
        (if (>= (`KismetArrayLibrary.Array_Length` (`self.SpawnedCharacters`)) 9)
          (`/Game/Characters/Pekorobo/BP_Character_Pekorobo.Death` (`|GetArrayItem` (`self.SpawnedCharacters`)))
          (`KismetArrayLibrary.Array_Remove` (`self.SpawnedCharacters`))))
      (:`then_1`
        (bind _returnvalue (`|SpawnActorFromClass` "/Game/Characters/Pekorobo/BP_Character_Pekorobo.BP_Character_Pekorobo_C" (`self.GetRandomSpawnTransform`) "AdjustIfPossibleButAlwaysSpawn" "OverrideRootScale" null null))
        (bind _returnvalue_2 (`self.K2_GetActorLocation` _returnvalue))
        (`NiagaraFunctionLibrary.SpawnSystemAtLocation` "/Game/Particles/NS_DustExplosion.NS_DustExplosion" _returnvalue_2 (struct) (0.5 0.5 0.5))
        (`GameplayStatics.SpawnSoundAtLocation` "/Game/Sounds/Expression_ClearPop.Expression_ClearPop" _returnvalue_2 (struct) 1.0 1.0 0.0 "/Game/Misc/PhysicsSound/Default/SA_Master.SA_Master" null)
        (`KismetArrayLibrary.Array_Add` (`self.SpawnedCharacters`) _returnvalue)))))

(fn `Change Cosmetic Pressed`
  (params (bPressed :type Boolean))
  (bind _asabp_button (cast `/Game/Actors/Button/ABP_Button` (`SkeletalMeshComponent.GetAnimInstance` (`self.SkeletalMesh`))))
  (bind _output_get (set `/Game/Actors/Button/ABP_Button.bPressed` bPressed _asabp_button))
  (if _output_get
    (`ActorComponent.Activate` (`self.SC_Button_Press`) true)
    (else
      (`ActorComponent.Activate` (`self.SC_Button_Release`) true))))

(fn `GetRandomSpawnTransform`
  (returns (ReturnValue :type "Transform Structure"))
  (bind (_origin _boxextent) (`KismetSystemLibrary.GetComponentBounds` (`self.Box1`)))
  (bind (_x _y) (`KismetMathLibrary.BreakVector3f` _boxextent))
  (return (`KismetMathLibrary.MakeTransform` (+ _origin (`KismetMathLibrary.MakeVector` (`KismetMathLibrary.RandomFloatInRange` (* _x -1.0) _x) (`KismetMathLibrary.RandomFloatInRange` (* _y -1.0) _y))) (`KismetMathLibrary.MakeRotator` 0.0 0.0 (`KismetMathLibrary.RandomFloatInRange` -180.0 180.0)) (0.5 0.5 0.5))))

(fn `IsCooldownOn`
  (returns (IsOn :type Boolean))
  (return (`KismetSystemLibrary.K2_IsValidTimerHandle` (`self.Timer`))))

(fn `OnCooldownExpired`
  (`KismetSystemLibrary.K2_ClearAndInvalidateTimerHandle` (`self.Timer`))
  (`self.Change Cosmetic Pressed` false))

(fn `SetCooldown`
  (bind _returnvalue (`KismetSystemLibrary.K2_SetTimerDelegate` (`|CreateDelegate` :!event `OnCooldownExpired`) (`self.Cooldown`)))
  (set `self.Timer` _returnvalue))

(fn `UserConstructionScript`
  (if (not true)
    (`TextRenderComponent.K2_SetText` (`self.Display`) (`KismetTextLibrary.Conv_StringToText` (`KismetStringLibrary.Concat_StrStr` "Play Dialogue" ":" (`KismetSystemLibrary.GetObjectName` null))))))