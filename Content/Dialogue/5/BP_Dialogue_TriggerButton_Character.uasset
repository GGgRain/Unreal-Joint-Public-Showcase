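; Overlap-triggered button that plays a dialogue joint using characters from a linked spawn button, with press animation and sound.
; On authority, a cooldown timer gates presses, which optionally end the previous joint, then create and start a new one.
; Before starting, spawned characters' participant components override the joint's participant fragments, matched by tag per index.
; TryPlaying returns true on every path, so AllowPlayingAgain never blocks replay.
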(event `self.Box.OnComponentBeginOverlap`
  (params (OverlappedComponent :type "PrimitiveComponent Object Reference") (OtherActor :type "Actor Object Reference") (OtherComp :type "PrimitiveComponent Object Reference") (OtherBodyIndex :type Integer) (bFromSweep :type Boolean) (SweepResult :type "HitResult Structure (by ref)"))
  (`|ExecutionSequence`
    (:`then_0`
      (`self.Change Cosmetic Pressed` true))
    (:`then_1`
      (if (`self.HasAuthority`)
        (if (not (`KismetSystemLibrary.K2_IsTimerActiveHandle` (`self.Timer`)))
          (bind _returnvalue (`KismetSystemLibrary.K2_SetTimerDelegate` (delegate `CustomEvent_0`) (`self.Cooldown`)))
          (set `self.Timer` _returnvalue)
          (`|ExecutionSequence`
            (:`then_0`
              (`self.Server_EndDialogue`))
            (:`then_1`
              (`self.Server_StartDialogue`))))))))

(event `CustomEvent_0`)

(event `self.Box.OnComponentEndOverlap`
  (params (OverlappedComponent :type "PrimitiveComponent Object Reference") (OtherActor :type "Actor Object Reference") (OtherComp :type "PrimitiveComponent Object Reference") (OtherBodyIndex :type Integer))
  (`self.Change Cosmetic Pressed` false))

(event `Server_EndDialogue`
  (`/Engine/EditorBlueprintResources/ActorMacros.Switch Has Authority`
    (:`Authority`
      (if (`self.bDestroyOldJointActorWhenPressed`)
        (`/Engine/EditorBlueprintResources/StandardMacros.IsValid` (`self.LastlyPlayedJointActor`)
          (:`Is Valid`
            (`JointActor.EndJoint` (`self.LastlyPlayedJointActor`))
            (set `self.LastlyPlayedJointActor` null)))))))

(event `Server_StartDialogue`
  (`/Engine/EditorBlueprintResources/ActorMacros.Switch Has Authority`
    (:`Authority`
      (if (`self.TryPlaying`)
        (bind _returnvalue (`JointSubsystem.CreateJoint` (`self.JointManagerToPlay`)))
        (bind _output_get (set `self.LastlyPlayedJointActor` _returnvalue))
        (`|ExecutionSequence`
          (:`then_0`
            (`self.Feed Overriden Participants` _output_get))
          (:`then_1`
            (`JointActor.StartJoint` _output_get)))))))

(fn `Change Cosmetic Pressed`
  (params (bPressed :type Boolean))
  (bind _asabp_button (cast `/Game/Actors/Button/ABP_Button` (`SkeletalMeshComponent.GetAnimInstance` (`self.SkeletalMesh`))))
  (set `/Game/Actors/Button/ABP_Button.bPressed` bPressed _asabp_button)
  (if bPressed
    (`ActorComponent.Activate` (`self.SC_Button_Press`) true)
    (else
      (`ActorComponent.Activate` (`self.SC_Button_Release`) true))))

(fn `Feed Overriden Participants`
  (params (`Joint Actor` :type "JointActor Object Reference"))
  (locals (CachedParticipants :type "Map of GameplayTag Structure to DF_Participant Object Reference") (TagsForIndices :type "Array of GameplayTag Structure"))
  (`|ExecutionSequence`
    (:`then_0`
      (for _array_element (`JointManager.FindManagerFragmentsByClassOnLowerHierarchy` (`JointActor.GetJointManager` `Joint Actor`) "/Script/JointNative.DF_Participant")
        (`BlueprintMapLibrary.Map_Add` (`local.CachedParticipants`) (`DF_Participant.ParticipantTag` _array_element) _array_element)))
    (:`then_1`
      (for (_array_element_2 _array_index) (`/Game/Dialogue/5/BP_CharacterSpawnButton.SpawnedCharacters` (`|ConvertAsset` (`self.CharacterSpawnButton`)))
        (bind (_value _returnvalue) (`BlueprintMapLibrary.Map_Find` (`local.CachedParticipants`) (`|GetArrayItem` (`local.TagsForIndices`) _array_index)))
        (if _returnvalue
          (set `DF_Participant.ParticipantComponentInstance` (`self.GetComponentByClass` _array_element_2 "/Script/JointNative.DialogueParticipantComponent") _value))))))

(fn `TryPlaying`
  (returns (CanPlay :type Boolean))
  (if (`self.bEverPlayed`)
    (if (`self.bAllowPlayingAgain`)
      _
      (else
        (return true))))
  (set `self.bEverPlayed` true)
  (return true))

(fn `UserConstructionScript`
  (if (not (`self.bUseCustomDisplayText`))
    (`TextRenderComponent.K2_SetText` (`self.Display`) (`KismetTextLibrary.Conv_StringToText` (`KismetStringLibrary.Concat_StrStr` "Play Dialogue" ":" (`KismetSystemLibrary.GetObjectName` (`self.JointManagerToPlay`)))))))